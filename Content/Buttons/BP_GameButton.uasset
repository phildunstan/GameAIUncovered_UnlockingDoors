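; Clickable game button actor that changes the color of its Cube mesh on cursor hover and click.
; BeginPlay creates a dynamic material from MI_GameButton; cursor events set the current and target colors.
; Hover snaps to the highlight color, while a click flashes the clicked color, which fades toward the current target.
; Tick eases toward the target using DeltaSeconds as lerp alpha and writes the Base Color parameter.
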(event MouseInput|EventActorOnClicked
  (params (ButtonPressed :type Key%20Structure))
  (Variables|Default|SetBase%20Color (Variables|Default|GetClicked%20Color)))

(event EventBeginPlay
  (Rendering|Material|CreateDynamicMaterialInstance (Variables|Default|GetCube) 0 "/Game/Buttons/MI_GameButton.MI_GameButton" "None" :!class /Script/Engine.PrimitiveComponent)
  (bind _output_get (Variables|Default|SetBase%20Color (Variables|Default|GetDefault%20Color)))
  (Variables|Default|SetTarget%20Color _output_get))

(event EventTick
  (params (DeltaSeconds :type Float%20%28single-precision%29))
  (bind _output_get (Variables|Default|SetBase%20Color (Math|Conversions|ToColor(LinearColor) (Math|Color|Lerp(LinearColor) (Math|Conversions|ToLinearColor(Color) (Variables|Default|GetBase%20Color)) (Math|Conversions|ToLinearColor(Color) (Variables|Default|GetTarget%20Color)) DeltaSeconds))))
  (Rendering|Material|SetColorParameterValueonMaterials (Variables|Default|GetCube) "Base Color" (Math|Conversions|ToLinearColor(Color) _output_get)))

(event MouseInput|EventActorBeginCursorOver
  (bind _output_get (Variables|Default|SetBase%20Color (Variables|Default|GetHighlighed%20Color)))
  (Variables|Default|SetTarget%20Color _output_get))

(event MouseInput|EventActorEndCursorOver
  (Variables|Default|SetTarget%20Color (Variables|Default|GetDefault%20Color)))

(fn ConstructionScript)