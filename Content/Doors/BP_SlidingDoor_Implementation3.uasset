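; Sliding door actor that opens, closes or toggles, and can start in the open state.
; A timeline slides the door mesh along the actor's local X axis from its closed position, ignoring commands while playing.
; When an agent reaches the nav link at a closed door, it stops, the door opens, and an On Door Open event resumes its path following.
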(event Custom|Handle%20On%20Door%20Open
  (EventDispatchers|UnbindEventfromOnDoorOpen (delegate Custom|Handle%20On%20Door%20Open))
  (Class|DoorwithNavLink|ResumePathFollowing (stale EventOnDoorNavLinkReached Agent)))

(event EventBeginPlay
  (Utilities|FlowControl|Sequence
    (:then_0
      (Variables|Default|SetClosedDoorPosition (Transformation|GetActorLocation)))
    (:then_1
      ;[0.15 0.15 0.15 0.5] Update the door position if the door starts open
      (if (Variables|Default|GetbIsOpen)
        (Components|Timeline|SetNewTime (Variables|Default|GetDoor%20Animation%20Timeline) 1e+02)))))

(event EventOpenDoor
  (if (not (Audio|Components|Audio|IsPlaying (Variables|Default|GetDoor%20Animation%20Timeline)))
    (if (not (Variables|Default|GetbIsOpen))
      (Audio|Components|Audio|Play (Variables|Default|GetDoor%20Animation%20Timeline)))))

(event EventCloseDoor
  (if (not (Audio|Components|Audio|IsPlaying (Variables|Default|GetDoor%20Animation%20Timeline)))
    (if (Variables|Default|GetbIsOpen)
      (Utilities|String|Reverse (Variables|Default|GetDoor%20Animation%20Timeline)))))

(event EventOnDoorNavLinkReached
  (params (Agent :type Actor%20Object%20Reference) (Destination :type Vector%20%28by%20ref%29 :default "0, 0, 0"))
  (if (not (Variables|Default|GetbIsOpen))
    (EventDispatchers|BindEventtoOnDoorOpen (delegate Custom|Handle%20On%20Door%20Open))
    (AI|Navigation|StopMovement (AI|GetAIController Agent))
    (Class|DoorInterface|OpenDoor)))

(event EventToggleDoorOpenorClosed
  (if (not (Audio|Components|Audio|IsPlaying (Variables|Default|GetDoor%20Animation%20Timeline)))
    (if (Variables|Default|GetbIsOpen)
      (Class|DoorInterface|CloseDoor)
      (else
        (Class|DoorInterface|OpenDoor)))))

(fn ConstructionScript)

(fn IsDoorOpen
  (return (Variables|Default|GetbIsOpen)))